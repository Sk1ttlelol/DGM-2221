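; A disappearing platform actor that reacts to the player stepping into its Box trigger.
; When a BP_PlayerPawn begins overlap, the Floor switches to a grass material, then after a delay turns invisible and loses collision.
; Any end overlap, with no pawn check, waits briefly, then restores the platform material and collision but sets visibility to false again, leaving the Floor solid yet hidden.
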(event OnComponentBeginOverlap(Box)
  (params (OverlappedComponent :type Primitive%20Component%20Object%20Reference) (OtherActor :type Actor%20Object%20Reference) (OtherComp :type Primitive%20Component%20Object%20Reference) (OtherBodyIndex :type Integer) (bFromSweep :type Boolean) (SweepResult :type Hit%20Result%20Structure%20%28by%20ref%29))
  (Utilities|Casting|CastToBP_PlayerPawn OtherActor)
  (Rendering|Material|SetMaterial (Variables|Default|GetFloor) 0 "/Game/StarterContent/Materials/M_Ground_Grass.M_Ground_Grass")
  (Utilities|FlowControl|Delay 3.0)
  (Rendering|SetVisibility (Variables|Default|GetFloor) false false)
  (Collision|SetCollisionEnabled (Variables|Default|GetFloor) "NoCollision"))

(event OnComponentEndOverlap(Box)
  (params (OverlappedComponent :type Primitive%20Component%20Object%20Reference) (OtherActor :type Actor%20Object%20Reference) (OtherComp :type Primitive%20Component%20Object%20Reference) (OtherBodyIndex :type Integer))
  (Utilities|FlowControl|Delay 1.0)
  (Rendering|Material|SetMaterial (Variables|Default|GetFloor) 0 "/Game/StarterContent/Materials/M_AssetPlatform.M_AssetPlatform")
  (Rendering|SetVisibility (Variables|Default|GetFloor) false false)
  (Collision|SetCollisionEnabled (Variables|Default|GetFloor) "QueryAndPhysics"))

(fn ConstructionScript)