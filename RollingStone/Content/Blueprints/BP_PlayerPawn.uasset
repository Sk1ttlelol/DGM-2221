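; BP_PlayerPawn is a physics-driven player pawn that rolls a RollingStone component and can push it vertically with a jetpack force.
; The forward/backward and left/right input axes apply torque around Y and X, while the Float Up axis applies force along Z.
; All inputs are scaled by tunable strength variables and applied as acceleration changes, so the response is independent of mass.
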(event Input|AxisEvents|InputAxisMoveForwards/Backwards
  (params (AxisValue :type Float%20%28single-precision%29))
  (Class|PrimitiveComponent|AddTorqueinRadians (Variables|Default|GetRollingStone) (Math|Vector|MakeVector 0.0 (* AxisValue (Variables|Default|GetTorqueStrength)) 0.0) "None" true))

(event Input|AxisEvents|InputAxisMoveLeft/Right
  (params (AxisValue :type Float%20%28single-precision%29))
  (Class|PrimitiveComponent|AddTorqueinRadians (Variables|Default|GetRollingStone) (Math|Vector|MakeVector (* AxisValue (Variables|Default|GetTorqueStrength)) 0.0 0.0) "None" true))

(event Input|AxisEvents|InputAxisFloatUp
  (params (AxisValue :type Float%20%28single-precision%29))
  (Physics|AddForce (Variables|Default|GetRollingStone) (Math|Vector|MakeVector 0.0 0.0 (* AxisValue (Variables|Default|GetJetPackForce))) "None" true))

(fn ConstructionScript)