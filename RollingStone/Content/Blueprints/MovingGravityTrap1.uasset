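; MovingGravityTrap1 is a trap that pulls the player's rolling stone toward its center.
; SphereCollider overlaps toggle a flag: any actor entering sets it, but only a BP_PlayerPawn leaving clears it.
; While the flag is set, Tick casts the overlapping actor to BP_PlayerPawn and applies a negative, constant-falloff radial force to its RollingStone as an acceleration change.
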(event OnComponentBeginOverlap(SphereCollider)
  (params (OverlappedComponent :type Primitive%20Component%20Object%20Reference) (OtherActor :type Actor%20Object%20Reference) (OtherComp :type Primitive%20Component%20Object%20Reference) (OtherBodyIndex :type Integer) (bFromSweep :type Boolean) (SweepResult :type Hit%20Result%20Structure%20%28by%20ref%29))
  (Variables|Default|SetBool true))

(event OnComponentEndOverlap(SphereCollider)
  (params (OverlappedComponent :type Primitive%20Component%20Object%20Reference) (OtherActor :type Actor%20Object%20Reference) (OtherComp :type Primitive%20Component%20Object%20Reference) (OtherBodyIndex :type Integer))
  (Utilities|Casting|CastToBP_PlayerPawn OtherActor)
  (Variables|Default|SetBool false))

(event EventTick
  (params (DeltaSeconds :type Float%20%28single-precision%29))
  (if (Variables|Default|GetBool)
    (bind _asbp_player_pawn (Utilities|Casting|CastToBP_PlayerPawn (stale OnComponentBeginOverlap(SphereCollider) OtherActor)))
    (Physics|AddRadialForce (Variables|/Game/Blueprints/BP_PlayerPawn.BP_PlayerPawn_C|GetRollingStone _asbp_player_pawn) (Transformation|GetActorLocation) 1e+04 -1e+04 "RIF_Constant" true)))

(fn ConstructionScript)