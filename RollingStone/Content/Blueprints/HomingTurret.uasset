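; HomingTurret is a turret actor that continuously tracks and shoots at the player's BP_PlayerPawn, cached on BeginPlay.
; Tick runs through a short Delay that throttles the loop, then turns the actor from its SpawnPoint toward the pawn's RollingStone component and spawns a Bullet.
; Each bullet's rotation leads the target, offsetting the aim by pawn velocity times distance over an assumed fixed bullet speed.
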(event EventBeginPlay
  (bind _asbp_player_pawn (Utilities|Casting|CastToBP_PlayerPawn (Game|Player|GetPlayerPawn 0)))
  (Variables|Default|SetPlayer%20Ref _asbp_player_pawn))

(event EventTick
  (params (DeltaSeconds :type Float%20%28single-precision%29))
  (bind _spawnpoint (Variables|Default|GetSpawnPoint))
  (bind _player_ref (Variables|Default|GetPlayer%20Ref))
  (bind _returnvalue (Transformation|GetWorldLocation _spawnpoint))
  (bind _rollingstone (Variables|/Game/Blueprints/BP_PlayerPawn.BP_PlayerPawn_C|GetRollingStone _player_ref))
  (bind _returnvalue_2 (Transformation|GetWorldLocation _rollingstone))
  (Utilities|FlowControl|Delay 0.1)
  (Transformation|SetActorRotation (Math|Rotator|FindLookatRotation _returnvalue _returnvalue_2))
  (Game|SpawnActorfromClass "/Game/Blueprints/Bullet.Bullet_C" (Math|Transform|MakeTransform _returnvalue (Math|Rotator|FindLookatRotation _returnvalue (+ _returnvalue_2 (* (Transformation|GetVelocity _player_ref) (/ (Transformation|GetDistanceTo _player_ref) 2e+03))))) "AdjustIfPossibleButAlwaysSpawn" 0 0))

(fn ConstructionScript)