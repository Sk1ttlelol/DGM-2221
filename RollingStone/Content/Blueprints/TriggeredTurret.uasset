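; A turret Blueprint that fires Bullet actors while something overlaps its Trigger component.
; Overlap begin and end on Trigger set and clear the TrueFalse flag, with no filtering by actor.
; A Delay on Tick acts as a five-second fire timer, checking the flag on completion and spawning a Bullet at SpawnPoint's world location and rotation.
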(event OnComponentBeginOverlap(Trigger)
  (params (OverlappedComponent :type Primitive%20Component%20Object%20Reference) (OtherActor :type Actor%20Object%20Reference) (OtherComp :type Primitive%20Component%20Object%20Reference) (OtherBodyIndex :type Integer) (bFromSweep :type Boolean) (SweepResult :type Hit%20Result%20Structure%20%28by%20ref%29))
  (Variables|Default|SetTrueFalse true))

(event OnComponentEndOverlap(Trigger)
  (params (OverlappedComponent :type Primitive%20Component%20Object%20Reference) (OtherActor :type Actor%20Object%20Reference) (OtherComp :type Primitive%20Component%20Object%20Reference) (OtherBodyIndex :type Integer))
  (Variables|Default|SetTrueFalse false))

(event EventTick
  (params (DeltaSeconds :type Float%20%28single-precision%29))
  (bind _spawnpoint (Variables|Default|GetSpawnPoint))
  (Utilities|FlowControl|Delay 5.0)
  (if (Variables|Default|GetTrueFalse)
    (Game|SpawnActorfromClass "/Game/Blueprints/Bullet.Bullet_C" (Math|Transform|MakeTransform (Transformation|GetWorldLocation _spawnpoint) (Transformation|GetWorldRotation _spawnpoint) "1,1,1") "AdjustIfPossibleButAlwaysSpawn" 0 0)))

(fn ConstructionScript)