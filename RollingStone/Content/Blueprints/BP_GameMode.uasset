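; BP_GameMode is a game mode Blueprint that respawns the player's pawn after it is destroyed.
; On BeginPlay it binds to the OnDestroyed event of player 0's BP_PlayerPawn.
; When that fires, it waits briefly, spawns a new pawn at the SpawnTransform variable and has the player controller possess it.
; It then calls Respawn to bind the new pawn, so the cycle repeats on each death.
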(event Custom|OnDestroyed_Event
  (params (DestroyedActor :type Actor%20Object%20Reference))
  ;[1 1 1] Death & Respawn
  (Utilities|FlowControl|Delay 2.0)
  (bind _returnvalue (Game|SpawnActorfromClass "/Game/Blueprints/BP_PlayerPawn.BP_PlayerPawn_C" (Variables|Default|GetSpawnTransform) "AdjustIfPossibleButAlwaysSpawn" 0 0))
  (Pawn|Possess (Game|GetPlayerController 0) _returnvalue)
  (CallFunction|Respawn))

(event Custom|Respawn
  ;[1 1 1] Death & Respawn
  (bind _asbp_player_pawn (Utilities|Casting|CastToBP_PlayerPawn (Game|Player|GetPlayerPawn 0)))
  (Game|BindEventtoOnDestroyed _asbp_player_pawn (delegate Custom|OnDestroyed_Event)))

(event EventBeginPlay
  ;[1 1 1] Death & Respawn
  (bind _asbp_player_pawn (Utilities|Casting|CastToBP_PlayerPawn (Game|Player|GetPlayerPawn 0)))
  (Game|BindEventtoOnDestroyed _asbp_player_pawn (delegate Custom|OnDestroyed_Event)))

(fn ConstructionScript)